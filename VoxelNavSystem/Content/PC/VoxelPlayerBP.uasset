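; VoxelPlayerBP is the player pawn for a voxel game, handling movement and a chunk-building action.
; On BeginPlay it adds the IMC_PlayerInput Enhanced Input mapping context to its player controller.
; IA_Move feeds its 2D value into the CharacterMovement input vector along world X and Y, independent of facing.
; IA_BuildChunk calls BuildChunkInCurrentPos, which is not defined in this graph.
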(event `self.ReceiveBeginPlay`
  (bind _returnvalue (`self.GetController`))
  (`/Engine/EditorBlueprintResources/StandardMacros.IsValid` _returnvalue
    (:`Is Valid`
      (bind `_as플레이어_컨트롤러` (cast `PlayerController` _returnvalue))
      (`EnhancedInputSubsystemInterface.AddMappingContext` (pcsubsystem `EnhancedInputLocalPlayerSubsystem` `_as플레이어_컨트롤러`) "/Game/Core/Input/IMC_PlayerInput.IMC_PlayerInput" 0 (struct)))))

(event `EnhancedInput|/Game/Core/Input/IA_Move`
  (params (ActionValue :type "Vector2D Structure") (ElapsedSeconds :type "Float (double-precision)") (TriggeredSeconds :type "Float (double-precision)") (InputAction :type "InputAction Object Reference" :default "/Game/Core/Input/IA_Move.IA_Move"))
  (bind (_x _y) (`KismetMathLibrary.BreakVector2D` ActionValue))
  (:`Triggered`
    (`PawnMovementComponent.AddInputVector` (`self.CharacterMovement`) (`KismetMathLibrary.MakeVector` _x _y) false)))

(event `EnhancedInput|/Game/Core/Input/IA_BuildChunk`
  (params (ActionValue :type Boolean) (ElapsedSeconds :type "Float (double-precision)") (TriggeredSeconds :type "Float (double-precision)") (InputAction :type "InputAction Object Reference" :default "/Game/Core/Input/IA_BuildChunk.IA_BuildChunk"))
  (:`Triggered`
    (`self.BuildChunkInCurrentPos`)))

(fn `UserConstructionScript`)